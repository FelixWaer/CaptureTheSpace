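; BP_PlayerSpaceShip is the player's spaceship Blueprint, handling HUD setup and shop menu opening.
; BeginPlay adds the main HUD to the viewport and sets a frame-rate cap through a console command.
; The shop input creates a new shop widget each time, showing the cursor and switching to UI-only input.
; It first checks the existing ShopRef's AllyVerticalBox enabled state, disabling the new widget when that is false.
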(event Input|EnhancedActionEvents|EnhancedInputActionIA_ShopOpen
  (params (ActionValue :type Boolean) (ElapsedSeconds :type Float%20%28double-precision%29) (TriggeredSeconds :type Float%20%28double-precision%29) (InputAction :type Input%20Action%20Object%20Reference :default "/Game/Input/InputActions/IA_ShopOpen.IA_ShopOpen"))
  (bind _returnvalue (Game|GetPlayerController 0))
  (bind _returnvalue_2 (Game|GetPlayerController 0))
  (:Started
    (if (Variables|/Script/UMG.Widget|GetbIsEnabled (Variables|/Game/Widgets/WBP_ShopWidget.WBP_ShopWidget_C|GetAlly_VerticalBox (Variables|Default|GetShopRef)))
      (bind _returnvalue_3 (UserInterface|CreateWidget "/Game/Widgets/WBP_ShopWidget.WBP_ShopWidget_C"))
      (Variables|Default|SetShopRef _returnvalue_3)
      (UserInterface|Viewport|AddtoViewport _returnvalue_3 0)
      (Variables|/Script/Engine.PlayerController|SetbShowMouseCursor _returnvalue true)
      (Input|SetInputModeUIOnly _returnvalue (Variables|Default|GetShopRef) "DoNotLock" false)
      (else
        (bind _returnvalue_4 (UserInterface|CreateWidget "/Game/Widgets/WBP_ShopWidget.WBP_ShopWidget_C"))
        (Variables|Default|SetShopRef _returnvalue_4)
        (UserInterface|Viewport|AddtoViewport _returnvalue_4 0)
        (Variables|/Script/Engine.PlayerController|SetbShowMouseCursor _returnvalue_2 true)
        (Input|SetInputModeUIOnly _returnvalue_2 (Variables|Default|GetShopRef) "DoNotLock" false)
        (Variables|/Script/UMG.Widget|SetbIsEnabled (Variables|Default|GetShopRef) false)))))

(event EventBeginPlay
  (CallFunction|AddHud)
  (Development|ExecuteConsoleCommand "t.maxfps 200" 0))

(event Collision|EventActorBeginOverlap
  (params (OtherActor :type Actor%20Object%20Reference)))

(event EventTick
  (params (DeltaSeconds :type Float%20%28single-precision%29)))

(fn ConstructionScript)

(fn AddHud
  (bind _returnvalue (UserInterface|CreateWidget "/Game/Widgets/WBP_MainHUD.WBP_MainHUD_C"))
  (UserInterface|Viewport|AddtoViewport _returnvalue 0))